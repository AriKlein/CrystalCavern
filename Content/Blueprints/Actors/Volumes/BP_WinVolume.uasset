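; BP_WinVolume is a level-completion volume that checks whether the player has collected every crystal on entering it.
; On player overlap, it prints either the remaining crystal count or a congratulations message with replay and quit prompts.
; AnyCrystalsRemaining counts live BP_Crystal actors, also gating the R and Q key events that restart the level or quit.
; CompleteLevel is an empty stub.
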(event `self.ReceiveActorBeginOverlap`
  (params (OtherActor :type "Actor Object Reference"))
  (bind (_numcrystalsremaining _crystalsremaining) (`self.Any_Crystals_Remaining`))
  (`/Game/Blueprints/Libraries/CC_MacroLibrary.isPlayer` OtherActor
    (:`isPlayer`
      (if _crystalsremaining
        (`KismetSystemLibrary.PrintString` (`KismetStringLibrary.Concat_StrStr` (`KismetStringLibrary.Concat_StrStr` "There are " (`KismetStringLibrary.Conv_IntToString` _numcrystalsremaining)) " Crystals Remaining."))
        (else
          (`KismetSystemLibrary.PrintString` "CONGRATS!! YOU GOT ALL THE CRYSTALS!")
          (`KismetSystemLibrary.PrintString` "Press CTRL+R to Replay or CTRL+Q to Quit")))
      (if (and (not _crystalsremaining) (== (stale `Key|R` Key) "R")) :!label _label
        (`/Game/Blueprints/Libraries/CC_MacroLibrary.RestartLevel`)))))

(event `Key|Q`
  (params (Key :type "Key Structure"))
  (:`Pressed`
    (if (and (not (`.crystalsRemaining` (`self.Any_Crystals_Remaining`))) (== Key "Q"))
      (`KismetSystemLibrary.QuitGame` null "Quit"))))

(event `Key|R`
  (params (Key :type "Key Structure"))
  (:`Pressed`
    (goto _label)))

(fn `Any_Crystals_Remaining`
  (returns (numCrystalsRemaining :type Integer) (crystalsRemaining :type Boolean))
  (bind _outactors (`GameplayStatics.GetAllActorsOfClass` "/Game/Blueprints/Actors/Collectibles/BP_Crystal.BP_Crystal_C"))
  (bind _returnvalue (`KismetArrayLibrary.Array_Length` _outactors))
  (return _returnvalue (> _returnvalue 0)))

(fn `Complete_Level`)

(fn `UserConstructionScript`)