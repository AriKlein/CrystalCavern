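; Cannon actor that automatically fires projectiles on a repeating cycle from BeginPlay.
; After a fire-rate delay, a timeline slides the turret along its local Y axis to animate the barrel.
; The timeline's Cannon Fired event spawns a scaled BP_Projectile at the spawn point, then loops back to the delay, so no Tick is needed.
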(event `self.ReceiveBeginPlay`
  (`KismetSystemLibrary.Delay` (`self.Cannon fire rate`) :!label _label)
  (bind (_direction _cannon_turret_rel_loc) (`Timeline|Cannon Fire Timeline` :!via `PlayFromStart`)
    (:`Update`
      (`self.MoveCannonBarrel` _cannon_turret_rel_loc))
    (:`Cannon Fired`
      (`self.Spawn Projectile`)
      (goto _label))))

(fn `MoveCannonBarrel`
  (params (`Cannon Barrel Y Location` :type "Float (double-precision)"))
  (`SceneComponent.K2_SetRelativeLocation` (`self.CannonTurret`) (`KismetMathLibrary.MakeVector` 0.0 `Cannon Barrel Y Location`) false false))

(fn `Spawn Projectile`
  (`|SpawnActorFromClass` "/Game/Blueprints/Actors/Projectiles/BP_Projectile.BP_Projectile_C" (`KismetMathLibrary.MakeTransform` (`SceneComponent.K2_GetComponentLocation` (`self.Projectile Spawn Point`)) (`SceneComponent.K2_GetComponentRotation` (`self.Projectile Spawn Point`)) (`KismetMathLibrary.Conv_DoubleToVector` (`self.Projectile Scale`))) "Undefined" "OverrideRootScale" null null))

(fn `UserConstructionScript`)