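; BP_Crystal is a collectible crystal that plays a collection animation and destroys itself when the player pawn overlaps it.
; On overlap it stores its starting location, scale and light intensity, then runs a timeline.
; Each update lerps the crystal toward the player's current position, shrinks it to zero scale and fades its light out, using separate timeline curves.
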(event `self.ReceiveActorBeginOverlap`
  (params (OtherActor :type "Actor Object Reference"))
  (`self.Is Player` OtherActor
    (:`is Player`
      (`self.Store Starting Crystal Values`)
      (bind (_direction _collection_progress _scale_progress _light_intensity) (`Timeline|collection timeline`)
        (:`Update`
          (`self.Move Crystal to Player` _collection_progress)
          (`self.Adjust light` _light_intensity)
          (`self.Scale crystal down` _scale_progress))
        (:`Finished`
          (`self.K2_DestroyActor`))))))

(fn `Adjust light`
  (params (Alpha :type "Float (double-precision)"))
  (`LightComponent.SetIntensity` (`self.CrystalLight`) (`KismetMathLibrary.Lerp` (`self.Lerp start light Intensity`) 0.0 Alpha)))

(fn `Move Crystal to Player`
  (params (Alpha :type "Float (double-precision)"))
  (`self.K2_SetActorLocation` (`KismetMathLibrary.VLerp` (`self.lerp start location`) (`self.K2_GetActorLocation` (`GameplayStatics.GetPlayerPawn` 0)) Alpha)))

(fn `Scale crystal down`
  (params (Alpha :type "Float (double-precision)"))
  (`self.SetActorScale3D` (`KismetMathLibrary.VLerp` (`self.Lerp start scale`) (0.0 0.0 0.0) Alpha)))

(fn `Store Starting Crystal Values`
  (locals (`start scale` :type "Vector Structure" :default (0.0 0.0 0.0)))
  (set `self.lerp start location` (`self.K2_GetActorLocation`))
  (set `self.Lerp start scale` (`self.GetActorScale3D`))
  (set `self.Lerp start light Intensity` (`LightComponentBase.Intensity` (`self.CrystalLight`))))

(fn `UserConstructionScript`)